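; BP_Semaforo is a traffic light actor that cycles endlessly from green to yellow to red, starting at a configurable light.
; ColorLights stores the current state, shows only the matching light component, then calls itself after that phase's delay.
; It also shows a Cube during yellow and red and hides it on green, always setting its collision to NoCollision.
; GetTrafficLight exposes the current state to other Blueprints.
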(event `self.ReceiveBeginPlay`
  (`self.ColorLights` (`self.Starting light`)))

(event `ColorLights`
  (params (EstadoSemaforo :type "/Game/IA_bp/Enums/EstadoSemaforo Enum" :default "NewEnumerator0"))
  (bind _output_get (set `self.EstadoSemaforo` EstadoSemaforo))
  (switch `/Game/IA_bp/Enums/EstadoSemaforo` _output_get
    (:`NewEnumerator0`
      (`self.ToggleGreenColors` true)
      (`self.ToggleYellowColors` false)
      (`self.ToggleRedColors` false)
      (`self.Toggle Cubes` false)
      (`KismetSystemLibrary.Delay` (`self.Duration`))
      (`self.ColorLights` "NewEnumerator1"))
    (:`NewEnumerator1`
      (`self.ToggleYellowColors` true)
      (`self.ToggleRedColors` false)
      (`self.ToggleGreenColors` false)
      (`self.Toggle Cubes` true)
      (`KismetSystemLibrary.Delay` (`self.Duration_0`))
      (`self.ColorLights` "NewEnumerator2"))
    (:`NewEnumerator2`
      (`self.ToggleRedColors` true)
      (`self.ToggleYellowColors` false)
      (`self.ToggleGreenColors` false)
      (`self.Toggle Cubes` true)
      (`KismetSystemLibrary.Delay` (`self.Duration_1`))
      (`self.ColorLights` "NewEnumerator0"))))

(fn `GetTrafficLight`
  (returns (NewParam :type "/Game/IA_bp/Enums/EstadoSemaforo Enum"))
  (return (`self.EstadoSemaforo`)))

(fn `Toggle Cubes`
  (params (on :type Boolean))
  (`SceneComponent.SetVisibility` (`self.Cube`) on false)
  (`PrimitiveComponent.SetCollisionEnabled` (`self.Cube`) "NoCollision"))

(fn `ToggleGreenColors`
  (params (On :type Boolean))
  (`SceneComponent.SetVisibility` (`self.green`) On false))

(fn `ToggleRedColors`
  (params (On :type Boolean))
  (`SceneComponent.SetVisibility` (`self.red`) On false))

(fn `ToggleYellowColors`
  (params (On :type Boolean))
  (`SceneComponent.SetVisibility` (`self.yellow`) On false))

(fn `UserConstructionScript`)